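; Heart actor that displays a flag and user name, with ID-checked events to set, hide or show it.
; BeginPlay gathers flag textures via the Asset Registry, and Set_Flag applies the name-matched one through a dynamic material instance.
; SetName spawns one text component per character and spaces them along a spline.
; ShowHeartInCube scales the heart up by timeline and starts a timer-driven sine yaw sway, which Stop clears while shrinking it.
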(event Custom|CustomEvent
  (bind _returnvalue (Utilities|Time|SetTimerbyEvent (delegate Custom|CustomEvent) 0.01 true))
  (bind _output_get (Variables|Default|SetRotation (Math|Float|Lerp 0.0 (Variables|Default|GetAmpl) (Math|Trig|Sin(Radians) (* (Utilities|Time|GetGameTimeinSeconds) (Variables|Default|GetSpeed))))))
  (Variables|Default|SetNewVar _returnvalue)
  (Transformation|SetRelativeRotation (Variables|Default|GetScene1) (Math|Rotator|MakeRotator 0.0 0.0 (+ (.Yaw (Math|Rotator|BreakRotator (Variables|Default|GetRotationStart))) (/ _output_get (Variables|Default|GetRotateZ)))) false false))

(event Custom|Set_Name
  (params (UserName :type String) (ID :type String))
  (if (Utilities|Enum|Equal(Enum) ID (Variables|Default|GetID))
    (CallFunction|SetName UserName)))

(event Custom|ShowHeartInCube
  (params (ID :type String))
  (if (Utilities|Enum|Equal(Enum) ID (Variables|Default|GetID))
    (Components|Timeline|SetPlayRate (Variables|Default|GetTimeline) (/ 1.0 (Variables|Default|GetHeartGrow)))
    (bind _newtrack_0 (Timeline|Timeline PlayFromStart)
      (:Update
        (Transformation|SetRelativeScale3D (Variables|Default|GetScene1) (Math|Vector|MakeVector (Math|Float|Lerp 0.01 1.0 _newtrack_0) (Math|Float|Lerp 0.01 1.0 _newtrack_0) (Math|Float|Lerp 0.01 1.0 _newtrack_0)))
        (CallFunction|CustomEvent)))))

(event Custom|Stop
  (Utilities|Time|ClearandInvalidateTimerbyHandle (Variables|Default|GetNewVar))
  (Transformation|SetRelativeScale3D (Variables|Default|GetScene1) "0.010000,0.010000,0.010000"))

(event Custom|Set_Flag
  (params (FlagName :type String) (ID :type String))
  (if (Utilities|Enum|Equal(Enum) ID (Variables|Default|GetID))
    (bind _output_get (Variables|Default|SetFlag%20Name FlagName))
    (CallFunction|SetTexture (Variables|Default|Getheart2upload) _output_get (Variables|Default|GetFragsTextureArray))
    (Development|PrintString _output_get true true "(R=0.000000,G=1.000000,B=0.013069,A=1.000000)" 3.0)
    (else
      (Development|PrintString "ErrorID" true true "(R=1.000000,G=0.000000,B=0.013838,A=1.000000)" 3.0))))

(event Custom|SetHidden
  (params (ID :type String) (bNewHidden :type Boolean))
  (if (Utilities|Enum|Equal(Enum) ID (Variables|Default|GetID))
    (Rendering|SetActorHiddenInGame bNewHidden)))

(event EventBeginPlay
  (CallFunction|GetTextureArray)
  (Input|EnableInput (Game|GetPlayerController 0)))

(event Input|KeyboardEvents|DebugKey1
  (params (Key :type Key%20Structure) (ActionValue :type Input%20Action%20Value%20Structure)))

(fn ConstructionScript)

(fn GetTextureArray
  (bind _outassetdata (Class|AssetRegistry|GetAssetsbyPath (Class|AssetRegistryHelpers|GetAssetRegistry) "/Game/Materials/Textures/Flags" true false))
  (for _array_element _outassetdata
    (bind _astexture_2d (Utilities|Casting|CastToTexture2D (Class|AssetRegistryHelpers|GetAsset _array_element)))
    (Utilities|Array|Add (Variables|Default|GetFragsTextureArray) _astexture_2d)))

(fn SetTexture
  (params (Mesh :type Primitive%20Component%20Object%20Reference) (FlagName :type String) (TextureArray :type Array%20of%20Texture%20Object%20References))
  (Utilities|FlowControl|Sequence
    (:then_0
      (bind _returnvalue (Rendering|Material|CreateDynamicMaterialInstance Mesh 0 "/Game/Materials/M_Flag_Inst.M_Flag_Inst" "None" :!class /Script/Engine.PrimitiveComponent))
      (bind (_array_element _array_index) (Utilities|Array|ForEachLoopwithBreak TextureArray :!label _label)
        (:LoopBody
          (if (Utilities|Enum|Equal(Enum) (Utilities|GetDisplayName _array_element) FlagName)
            (Utilities|FlowControl|Sequence
              (:then_0
                (Rendering|Material|SetTextureParameterValue _returnvalue "Flag" (Utilities|Array|Get(acopy) TextureArray _array_index)))
              (:then_1
                (goto _label Break)))))))))

(fn SetName
  (params (UserName :type String) (Spline :type Spline%20Component%20Object%20Reference))
  (bind _spline1 (Variables|Default|GetSpline1))
  (bind _letter (Variables|Default|GetLetter))
  (bind _spline1_2 (Variables|Default|GetSpline1))
  (bind _returnvalue (Utilities|Array|Length _letter))
  (bind _returnvalue_2 (Spline|GetSplineLength _spline1))
  (for _array_element (Utilities|String|GetCharacterArrayfromString UserName)
    (bind _returnvalue_3 (AddComponent|AddTextRenderComponent false))
    (Class|TextRenderComponent|SetTextMaterial _returnvalue_3 "/Game/BP/Fonts/DefaultTextMaterialOpaque1.DefaultTextMaterialOpaque1")
    (Class|TextRenderComponent|SetFont _returnvalue_3 "/Game/BP/Fonts/TT_Norms_Pro_Trial_Medium.TT_Norms_Pro_Trial_Medium")
    (Rendering|Components|TextRender|SetWorldSize _returnvalue_3 (Variables|Default|GetTextSize))
    (Rendering|Components|SetLightingChannels _returnvalue_3 false true false)
    (Utilities|Array|Add (Variables|Default|GetLetter) _returnvalue_3)
    (Rendering|Components|TextRender|SetText _returnvalue_3 (Utilities|Text|ToText(String) _array_element)))
  (for (_array_element_2 _array_index) _letter
    (if (<= _returnvalue 5)
      (Variables|Default|SetStep 0.15)
      (elif (>= _returnvalue 12)
        (Variables|Default|SetStep 0.3)))
    (bind _output_get (Variables|Default|SetDistanceAlongSpline (+ (* (- _array_index (/ (+ _returnvalue -1) 2)) (* (/ _returnvalue_2 _returnvalue) (Variables|Default|GetStep))) (/ _returnvalue_2 2.0))))
    (if (> _output_get (* (/ _returnvalue_2 _returnvalue) (Variables|Default|GetStep)))
      (Variables|Default|SetDistanceAlongSpline (- (Variables|Default|GetDistanceAlongSpline) (* (/ _returnvalue_2 _returnvalue) (Variables|Default|GetStep)))))
    (Transformation|SetWorldLocationAndRotation _array_element_2 (Spline|GetLocationatDistanceAlongSpline _spline1_2 (Variables|Default|GetDistanceAlongSpline) "World") (Math|Rotator|CombineRotators (Spline|GetRotationatDistanceAlongSpline _spline1_2 (Variables|Default|GetDistanceAlongSpline) "World") (Variables|Default|GetRotator)) false false)))