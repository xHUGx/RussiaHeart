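; Heart actor that displays a country or other flag on its mesh and a user name curved along a spline.
; On BeginPlay it loads textures from the Flags folder via the Asset Registry; Set_Texture matches one by name and applies it through a dynamic material instance.
; SetName, run from the construction script and Set_Name event, creates one TextRender component per character, spacing them around the spline's midpoint.
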(event Custom|Set_Texture
  (params (FlagName :type String))
  (CallFunction|SetTexture (Variables|Default|Getheart2upload) FlagName (Variables|Default|GetFragsTextureArray)))

(event Custom|Set_Name
  (params (UserName :type String))
  (CallFunction|SetName UserName (Variables|Default|GetSpline)))

(event EventBeginPlay
  (CallFunction|GetTextureArray))

(fn ConstructionScript
  (CallFunction|SetName (Variables|Default|GetUser%20Name) (Variables|Default|GetSpline)))

(fn GetTextureArray
  (bind _outassetdata (Class|AssetRegistry|GetAssetsbyPath (Class|AssetRegistryHelpers|GetAssetRegistry) "/Game/Materials/Textures/Flags" true false))
  (for _array_element _outassetdata
    (bind _astexture_2d (Utilities|Casting|CastToTexture2D (Class|AssetRegistryHelpers|GetAsset _array_element)))
    (Utilities|Array|Add (Variables|Default|GetFragsTextureArray) _astexture_2d)))

(fn SetTexture
  (params (Mesh :type Primitive%20Component%20Object%20Reference) (FlagName :type String) (TextureArray :type Array%20of%20Texture%20Object%20References))
  (Utilities|FlowControl|Sequence
    (:then_0
      (bind _returnvalue (Rendering|Material|CreateDynamicMaterialInstance Mesh 0 "/Game/Materials/M_Flag_Inst.M_Flag_Inst" "None" :!class /Script/Engine.PrimitiveComponent))
      (bind (_array_element _array_index) (Utilities|Array|ForEachLoopwithBreak TextureArray :!label _label)
        (:LoopBody
          (if (Utilities|Enum|Equal(Enum) (Utilities|GetDisplayName _array_element) FlagName)
            (Utilities|FlowControl|Sequence
              (:then_0
                (Rendering|Material|SetTextureParameterValue _returnvalue "Flag" (Utilities|Array|Get(acopy) TextureArray _array_index)))
              (:then_1
                (goto _label Break)))))))))

(fn SetName
  (params (UserName :type String) (Spline :type Spline%20Component%20Object%20Reference))
  (bind _step (Variables|Default|GetStep))
  (bind _letter (Variables|Default|GetLetter))
  (bind _returnvalue (Utilities|Array|Length _letter))
  (bind _returnvalue_2 (Spline|GetSplineLength (Variables|Default|GetSpline)))
  (bind _returnvalue_3 (/ _returnvalue_2 _returnvalue))
  (bind _returnvalue_4 (* _returnvalue_3 _step))
  (for _array_element (Utilities|String|GetCharacterArrayfromString UserName)
    (bind _returnvalue_5 (AddComponent|AddTextRenderComponent false))
    (Class|TextRenderComponent|SetTextMaterial _returnvalue_5 "/Game/BP/Fonts/DefaultTextMaterialOpaque1.DefaultTextMaterialOpaque1")
    (Class|TextRenderComponent|SetFont _returnvalue_5 "/Game/BP/Fonts/TT_Norms_Pro_Trial_Medium.TT_Norms_Pro_Trial_Medium")
    (Rendering|Components|TextRender|SetWorldSize _returnvalue_5 (Variables|Default|GetTextSize))
    (Rendering|Components|SetLightingChannels _returnvalue_5 false true false)
    (Utilities|Array|Add (Variables|Default|GetLetter) _returnvalue_5)
    (Rendering|Components|TextRender|SetText _returnvalue_5 (Utilities|Text|ToText(String) _array_element)))
  (for (_array_element_2 _array_index) _letter
    (bind _output_get (Variables|Default|SetDistanceAlongSpline (+ (* (- _array_index (/ (+ _returnvalue -1) 2)) _returnvalue_4) (/ _returnvalue_2 2.0))))
    (if (> _output_get _returnvalue_4)
      (Variables|Default|SetDistanceAlongSpline (- (Variables|Default|GetDistanceAlongSpline) _returnvalue_4)))
    (Transformation|SetWorldLocationAndRotation _array_element_2 (Spline|GetLocationatDistanceAlongSpline (Variables|Default|GetSpline) (Variables|Default|GetDistanceAlongSpline) "World") (Math|Rotator|CombineRotators (Spline|GetRotationatDistanceAlongSpline (Variables|Default|GetSpline) (Variables|Default|GetDistanceAlongSpline) "World") (Variables|Default|GetRotator)) false false)))