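; OSC server actor that drives eight heart actor classes from remote messages, listening on a hard-coded IP and port.
; It stores incoming flag and ID strings; a name message pushes all three values to BP_Heart01–08, setting flag and name and showing the heart in the cube.
; A start message plays the _HeartMovement02 Level Sequence.
; A stop message stops the hearts, clears the name and destroys the sequence actor.
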(event Custom|OSCMessengeRecived
  (params (Message :type OSC%20Message%20Structure%20%28by%20ref%29) (IPAddress :type String) (Port :type Integer))
  (bind _returnvalue (Class|OSCManager|GetOSCMessageAddress Message))
  (bind _returnvalue_2 (Class|OSCManager|GetOSCAddressFullPath _returnvalue))
  (Utilities|FlowControl|Sequence
    (:then_0
      (if (Class|KismetStringLibrary|MatchesWildcard _returnvalue_2 "/name" "IgnoreCase")
        (bind _value (Class|OSCManager|GetString Message))
        (bind _output_get (Variables|Default|SetName _value))
        (Development|PrintString _output_get)
        (Utilities|FlowControl|Sequence
          (:then_0
            (CallFunction|Heart01 (Variables|Default|GetFlag) (Variables|Default|GetID) (Variables|Default|GetName) (Variables|Default|GetNew%20Hidden)))
          (:then_1
            (CallFunction|Heart02 (Variables|Default|GetFlag) (Variables|Default|GetID) (Variables|Default|GetName) (Variables|Default|GetNew%20Hidden)))
          (:then_2
            (CallFunction|Heart03 (Variables|Default|GetFlag) (Variables|Default|GetID) (Variables|Default|GetName) (Variables|Default|GetNew%20Hidden)))
          (:then_3
            (CallFunction|Heart04 (Variables|Default|GetFlag) (Variables|Default|GetID) (Variables|Default|GetName) (Variables|Default|GetNew%20Hidden)))
          (:then_4
            (CallFunction|Heart05 (Variables|Default|GetFlag) (Variables|Default|GetID) (Variables|Default|GetName) (Variables|Default|GetNew%20Hidden)))
          (:then_5
            (CallFunction|Heart06 (Variables|Default|GetFlag) (Variables|Default|GetID) (Variables|Default|GetName) (Variables|Default|GetNew%20Hidden)))
          (:then_6
            (CallFunction|Heart07 (Variables|Default|GetFlag) (Variables|Default|GetID) (Variables|Default|GetName) (Variables|Default|GetNew%20Hidden)))
          (:then_7
            (CallFunction|Heart08 (Variables|Default|GetFlag) (Variables|Default|GetID) (Variables|Default|GetName) (Variables|Default|GetNew%20Hidden))))))
    (:then_1
      (if (Class|KismetStringLibrary|MatchesWildcard _returnvalue_2 "/flag" "IgnoreCase")
        (bind _value_2 (Class|OSCManager|GetString Message))
        (bind _output_get_2 (Variables|Default|SetFlag _value_2))
        (Development|PrintString _output_get_2)))
    (:then_2
      (if (Class|KismetStringLibrary|MatchesWildcard _returnvalue_2 "/Id" "IgnoreCase")
        (bind _value_3 (Class|OSCManager|GetString Message))
        (bind _output_get_3 (Variables|Default|SetID _value_3))
        (Development|PrintString _output_get_3)))
    (:then_3
      (if (Class|KismetStringLibrary|MatchesWildcard _returnvalue_2 "/start" "IgnoreCase")
        (bind _outactor (Sequencer|Player|CreateLevelSequencePlayer "/Game/Sequence/_HeartMovement02._HeartMovement02"))
        (Sequencer|Player|Play (Variables|/Script/LevelSequence.LevelSequenceActor|GetSequencePlayer _outactor) :!class /Script/MovieScene.MovieSceneSequencePlayer)
        (else
          (Development|PrintString "SequenceNone" true true "(R=1.000000,G=0.000000,B=0.031298,A=1.000000)"))))
    (:then_4
      (if (Class|KismetStringLibrary|MatchesWildcard _returnvalue_2 "/stop" "IgnoreCase")
        (Utilities|FlowControl|Sequence
          (:then_0
            (bind _outactors (Actor|GetAllActorsOfClass "/Game/BP/UniqHearts/BP_Heart01.BP_Heart01_C"))
            (Default|Stop _outactors))
          (:then_1
            (bind _outactors_2 (Actor|GetAllActorsOfClass "/Game/BP/UniqHearts/BP_Heart02.BP_Heart02_C"))
            (Default|Stop _outactors_2))
          (:then_2
            (bind _outactors_3 (Actor|GetAllActorsOfClass "/Game/BP/UniqHearts/BP_Heart03.BP_Heart03_C"))
            (Default|Stop _outactors_3))
          (:then_3
            (bind _outactors_4 (Actor|GetAllActorsOfClass "/Game/BP/UniqHearts/BP_Heart04.BP_Heart04_C"))
            (Default|Stop _outactors_4))
          (:then_4
            (bind _outactors_5 (Actor|GetAllActorsOfClass "/Game/BP/UniqHearts/BP_Heart05.BP_Heart05_C"))
            (Default|Stop _outactors_5))
          (:then_5
            (bind _outactors_6 (Actor|GetAllActorsOfClass "/Game/BP/UniqHearts/BP_Heart06.BP_Heart06_C"))
            (Default|Stop _outactors_6))
          (:then_6
            (bind _outactors_7 (Actor|GetAllActorsOfClass "/Game/BP/UniqHearts/BP_Heart07.BP_Heart07_C"))
            (Default|Stop _outactors_7))
          (:then_7
            (bind _outactors_8 (Actor|GetAllActorsOfClass "/Game/BP/UniqHearts/BP_Heart08.BP_Heart08_C"))
            (Default|Stop _outactors_8)))
        (Variables|Default|SetName "")
        (Actor|DestroyActor _outactor)))))

(event EventBeginPlay
  (bind _returnvalue (Class|OSCManager|CreateOSCServer "192.168.2.95" 7000 false true "" 0))
  (bind _output_get (Variables|Default|SetOSCServer _returnvalue))
  (EventDispatchers|UnbindallEventsfromOnOscBundleReceived _output_get)
  (EventDispatchers|BindEventtoOnOscMessageReceived _output_get (EventDispatchers|CreateEvent :!event Custom|OSCMessengeRecived)))

(fn ConstructionScript)

(fn Heart01
  (params (FlagName :type String) (ID :type String) (UserName :type String) (bNewHidden :type Boolean))
  (bind _outactors (Actor|GetAllActorsOfClass "/Game/BP/UniqHearts/BP_Heart01.BP_Heart01_C"))
  (Default|SetFlag _outactors FlagName ID)
  (Default|SetName _outactors UserName ID)
  (Default|ShowHeartinCube _outactors ID))

(fn Heart02
  (params (FlagName :type String) (ID :type String) (UserName :type String) (bNewHidden :type Boolean))
  (bind _outactors (Actor|GetAllActorsOfClass "/Game/BP/UniqHearts/BP_Heart02.BP_Heart02_C"))
  (Default|SetFlag _outactors FlagName ID)
  (Default|SetName _outactors UserName ID)
  (Default|ShowHeartinCube _outactors ID))

(fn Heart03
  (params (FlagName :type String) (ID :type String) (UserName :type String) (bNewHidden :type Boolean))
  (bind _outactors (Actor|GetAllActorsOfClass "/Game/BP/UniqHearts/BP_Heart03.BP_Heart03_C"))
  (Default|SetFlag _outactors FlagName ID)
  (Default|SetName _outactors UserName ID)
  (Default|ShowHeartinCube _outactors ID))

(fn Heart04
  (params (FlagName :type String) (ID :type String) (UserName :type String) (bNewHidden :type Boolean))
  (bind _outactors (Actor|GetAllActorsOfClass "/Game/BP/UniqHearts/BP_Heart04.BP_Heart04_C"))
  (Default|SetFlag _outactors FlagName ID)
  (Default|SetName _outactors UserName ID)
  (Default|ShowHeartinCube _outactors ID))

(fn Heart05
  (params (FlagName :type String) (ID :type String) (UserName :type String) (bNewHidden :type Boolean))
  (bind _outactors (Actor|GetAllActorsOfClass "/Game/BP/UniqHearts/BP_Heart05.BP_Heart05_C"))
  (Default|SetFlag _outactors FlagName ID)
  (Default|SetName _outactors UserName ID)
  (Default|ShowHeartinCube _outactors ID))

(fn Heart06
  (params (FlagName :type String) (ID :type String) (UserName :type String) (bNewHidden :type Boolean))
  (bind _outactors (Actor|GetAllActorsOfClass "/Game/BP/UniqHearts/BP_Heart06.BP_Heart06_C"))
  (Default|SetFlag _outactors FlagName ID)
  (Default|SetName _outactors UserName ID)
  (Default|ShowHeartinCube _outactors ID))

(fn Heart07
  (params (FlagName :type String) (ID :type String) (UserName :type String) (bNewHidden :type Boolean))
  (bind _outactors (Actor|GetAllActorsOfClass "/Game/BP/UniqHearts/BP_Heart07.BP_Heart07_C"))
  (Default|SetFlag _outactors FlagName ID)
  (Default|SetName _outactors UserName ID)
  (Default|ShowHeartinCube _outactors ID))

(fn Heart08
  (params (FlagName :type String) (ID :type String) (UserName :type String) (bNewHidden :type Boolean))
  (bind _outactors (Actor|GetAllActorsOfClass "/Game/BP/UniqHearts/BP_Heart08.BP_Heart08_C"))
  (Default|SetFlag _outactors FlagName ID)
  (Default|SetName _outactors UserName ID)
  (Default|ShowHeartinCube _outactors ID))