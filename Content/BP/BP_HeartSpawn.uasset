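; BP_HeartSpawn spawns BP_Heart1 actors attached to itself, each showing a country flag and, in most cases, a person's name.
; SpawnHeart01 takes a flag name; the other seven events hard-code "ua" and a name.
; GetTextureArray appends flag textures found through the Asset Registry, and SetTexture applies the name match via a dynamic material.
; SetName lays per-character text components along the heart's spline, using a shared, never-cleared Letter array.
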(event Custom|SpawnHeart08
  (bind _returnvalue (Game|SpawnActorfromClass "/Game/BP/BP_Heart1.BP_Heart1_C" (Variables|Default|GetSpawn%20Transform) "Undefined" "MultiplyWithRoot" 0 0))
  (Transformation|AttachActorToActor _returnvalue self "None" "KeepRelative" "KeepRelative" "KeepRelative" true)
  (CallFunction|GetTextureArray)
  (CallFunction|SetTexture (Variables|/Game/BP/BP_Heart1.BP_Heart1_C|Getheart2upload _returnvalue) "ua" (Variables|Default|GetFragsTextureArray))
  (CallFunction|SetName "Игорь Гофман" (Variables|/Game/BP/BP_Heart1.BP_Heart1_C|GetSpline _returnvalue)))

(event Custom|SpawnHeart01
  (params (FlagName :type String))
  (bind _returnvalue (Game|SpawnActorfromClass "/Game/BP/BP_Heart1.BP_Heart1_C" (Variables|Default|GetSpawn%20Transform) "Undefined" "MultiplyWithRoot" 0 0))
  (Transformation|AttachActorToActor _returnvalue self "None" "KeepRelative" "KeepRelative" "KeepRelative" true)
  (Utilities|FlowControl|Sequence
    (:then_0
      (CallFunction|GetTextureArray)
      (CallFunction|SetTexture (Variables|/Game/BP/BP_Heart1.BP_Heart1_C|Getheart2upload _returnvalue) FlagName (Variables|Default|GetFragsTextureArray)))))

(event Custom|SpawnHeart06
  (bind _returnvalue (Game|SpawnActorfromClass "/Game/BP/BP_Heart1.BP_Heart1_C" (Variables|Default|GetSpawn%20Transform) "Undefined" "MultiplyWithRoot" 0 0))
  (Transformation|AttachActorToActor _returnvalue self "None" "KeepRelative" "KeepRelative" "KeepRelative" true)
  (CallFunction|GetTextureArray)
  (CallFunction|SetTexture (Variables|/Game/BP/BP_Heart1.BP_Heart1_C|Getheart2upload _returnvalue) "ua" (Variables|Default|GetFragsTextureArray))
  (CallFunction|SetName "Игорь Гофман" (Variables|/Game/BP/BP_Heart1.BP_Heart1_C|GetSpline _returnvalue)))

(event Custom|SpawnHeart07
  (bind _returnvalue (Game|SpawnActorfromClass "/Game/BP/BP_Heart1.BP_Heart1_C" (Variables|Default|GetSpawn%20Transform) "Undefined" "MultiplyWithRoot" 0 0))
  (Transformation|AttachActorToActor _returnvalue self "None" "KeepRelative" "KeepRelative" "KeepRelative" true)
  (CallFunction|GetTextureArray)
  (CallFunction|SetTexture (Variables|/Game/BP/BP_Heart1.BP_Heart1_C|Getheart2upload _returnvalue) "ua" (Variables|Default|GetFragsTextureArray))
  (CallFunction|SetName "Игорь Гофман" (Variables|/Game/BP/BP_Heart1.BP_Heart1_C|GetSpline _returnvalue)))

(event Custom|SpawnHeart02
  (bind _returnvalue (Game|SpawnActorfromClass "/Game/BP/BP_Heart1.BP_Heart1_C" (Variables|Default|GetSpawn%20Transform) "Undefined" "MultiplyWithRoot" 0 0))
  (Utilities|IsValid _returnvalue
    (:Is%20Valid
      (Transformation|AttachActorToActor _returnvalue self "None" "KeepRelative" "KeepRelative" "KeepRelative" true)
      (CallFunction|GetTextureArray)
      (CallFunction|SetTexture (Variables|/Game/BP/BP_Heart1.BP_Heart1_C|Getheart2upload _returnvalue) "ua" (Variables|Default|GetFragsTextureArray))
      (CallFunction|SetName "Григорий" (Variables|/Game/BP/BP_Heart1.BP_Heart1_C|GetSpline _returnvalue)))
    (:Is%20Not%20Valid
      (Development|PrintString "ActorDestroyed"))))

(event Custom|SpawnHeart03
  (bind _returnvalue (Game|SpawnActorfromClass "/Game/BP/BP_Heart1.BP_Heart1_C" (Variables|Default|GetSpawn%20Transform) "Undefined" "MultiplyWithRoot" 0 0))
  (Transformation|AttachActorToActor _returnvalue self "None" "KeepRelative" "KeepRelative" "KeepRelative" true)
  (CallFunction|GetTextureArray)
  (CallFunction|SetTexture (Variables|/Game/BP/BP_Heart1.BP_Heart1_C|Getheart2upload _returnvalue) "ua" (Variables|Default|GetFragsTextureArray))
  (CallFunction|SetName "Шепард" (Variables|/Game/BP/BP_Heart1.BP_Heart1_C|GetSpline _returnvalue)))

(event Custom|SpawnHeart04
  (bind _returnvalue (Game|SpawnActorfromClass "/Game/BP/BP_Heart1.BP_Heart1_C" (Variables|Default|GetSpawn%20Transform) "Undefined" "MultiplyWithRoot" 0 0))
  (Transformation|AttachActorToActor _returnvalue self "None" "KeepRelative" "KeepRelative" "KeepRelative" true)
  (CallFunction|GetTextureArray)
  (CallFunction|SetTexture (Variables|/Game/BP/BP_Heart1.BP_Heart1_C|Getheart2upload _returnvalue) "ua" (Variables|Default|GetFragsTextureArray))
  (CallFunction|SetName "Просто клевый парень" (Variables|/Game/BP/BP_Heart1.BP_Heart1_C|GetSpline _returnvalue)))

(event Custom|SpawnHeart05
  (bind _returnvalue (Game|SpawnActorfromClass "/Game/BP/BP_Heart1.BP_Heart1_C" (Variables|Default|GetSpawn%20Transform) "Undefined" "MultiplyWithRoot" 0 0))
  (Transformation|AttachActorToActor _returnvalue self "None" "KeepRelative" "KeepRelative" "KeepRelative" true)
  (CallFunction|GetTextureArray)
  (CallFunction|SetTexture (Variables|/Game/BP/BP_Heart1.BP_Heart1_C|Getheart2upload _returnvalue) "ua" (Variables|Default|GetFragsTextureArray))
  (CallFunction|SetName "Игорь Гофман" (Variables|/Game/BP/BP_Heart1.BP_Heart1_C|GetSpline _returnvalue)))

(fn ConstructionScript)

(fn GetTextureArray
  (bind _outassetdata (Class|AssetRegistry|GetAssetsbyPath (Class|AssetRegistryHelpers|GetAssetRegistry) "/Game/Materials/Textures/Flags" true false))
  (for _array_element _outassetdata
    (bind _astexture_2d (Utilities|Casting|CastToTexture2D (Class|AssetRegistryHelpers|GetAsset _array_element)))
    (Utilities|Array|Add (Variables|Default|GetFragsTextureArray) _astexture_2d)))

(fn SetTexture
  (params (Mesh :type Primitive%20Component%20Object%20Reference) (FlagName :type String) (TextureArray :type Array%20of%20Texture%20Object%20References))
  (Utilities|FlowControl|Sequence
    (:then_0
      (bind _returnvalue (Rendering|Material|CreateDynamicMaterialInstance Mesh 0 "/Game/Materials/M_Flag_Inst.M_Flag_Inst" "None" :!class /Script/Engine.PrimitiveComponent))
      (bind (_array_element _array_index) (Utilities|Array|ForEachLoopwithBreak TextureArray :!label _label)
        (:LoopBody
          (if (Utilities|Enum|Equal(Enum) (Utilities|GetDisplayName _array_element) FlagName)
            (Utilities|FlowControl|Sequence
              (:then_0
                (Rendering|Material|SetTextureParameterValue _returnvalue "Flag" (Utilities|Array|Get(acopy) TextureArray _array_index)))
              (:then_1
                (goto _label Break)))))))))

(fn SetName
  (params (UserName :type String) (Spline :type Spline%20Component%20Object%20Reference))
  (bind _letter (Variables|Default|GetLetter))
  (for _array_element (Utilities|String|GetCharacterArrayfromString UserName)
    (bind _returnvalue (AddComponent|AddTextRenderComponent false))
    (Class|TextRenderComponent|SetTextMaterial _returnvalue "/Game/BP/Fonts/DefaultTextMaterialOpaque1.DefaultTextMaterialOpaque1")
    (Class|TextRenderComponent|SetFont _returnvalue "/Game/BP/Fonts/TT_Norms_Pro_Compact_Trial_Black.TT_Norms_Pro_Compact_Trial_Black")
    (Rendering|Components|TextRender|SetWorldSize _returnvalue (Variables|Default|GetTextSize))
    (Rendering|Components|SetLightingChannels _returnvalue false true false)
    (Utilities|Array|Add (Variables|Default|GetLetter) _returnvalue)
    (Rendering|Components|TextRender|SetText _returnvalue (Utilities|Text|ToText(String) _array_element)))
  (for (_array_element_2 _array_index) _letter
    (Transformation|SetWorldLocationAndRotation _array_element_2 (Spline|GetLocationatDistanceAlongSpline (Variables|Default|GetSpline) (* (* (Math|Conversions|ToFloat(Integer) _array_index) (/ (Spline|GetSplineLength (Variables|Default|GetSpline)) (Math|Conversions|ToFloat(Integer) (Utilities|Array|Length _letter)))) (Variables|Default|GetSpacing)) "World") (Math|Rotator|CombineRotators (Spline|GetRotationatDistanceAlongSpline (Variables|Default|GetSpline) (* (* (Math|Conversions|ToFloat(Integer) _array_index) (/ (Spline|GetSplineLength (Variables|Default|GetSpline)) (Math|Conversions|ToFloat(Integer) (Utilities|Array|Length _letter)))) (Variables|Default|GetSpacing)) "World") (Variables|Default|GetRotator)) false false)))